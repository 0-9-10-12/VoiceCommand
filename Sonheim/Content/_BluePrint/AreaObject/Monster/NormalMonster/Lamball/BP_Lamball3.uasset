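; Lamball monster variant that seeks a nearby resource object on spawn and can switch facial expressions.
; The construction script creates per-instance dynamic materials for the eye and mouth slots.
; ChangeFace copies expression vectors from the eye and mouth parameter collections into those materials, so each Lamball's face changes independently.
; BeginPlay calls GetNearResourceObject with a random argument; leftover face-test and rock-target nodes are unconnected.
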(event `self.ReceiveBeginPlay`
  (`self.GetNearResourceObject` (* (`KismetMathLibrary.RandomIntegerInRange` 0 2) 5)))

(event `self.ChangeFace`
  (params (Feel :type Integer))
  (switch `int` Feel
    (:`0`
      (bind _returnvalue (`KismetMaterialLibrary.GetVectorParameterValue` "/Game/_Resource/Monster/Lamball/MPC_Mouth.MPC_Mouth" "Smile"))
      (bind _returnvalue_2 (`KismetMaterialLibrary.GetVectorParameterValue` "/Game/_Resource/Monster/Lamball/MPC_Eye.MPC_Eye" "Smile"))
      (`MaterialInstanceDynamic.SetVectorParameterValue` (`self.MouseMaterial`) "Mouth" _returnvalue)
      (`MaterialInstanceDynamic.SetVectorParameterValue` (`self.EyeMaterial`) "Eye" _returnvalue_2))
    (:`1`
      (bind _returnvalue_3 (`KismetMaterialLibrary.GetVectorParameterValue` "/Game/_Resource/Monster/Lamball/MPC_Mouth.MPC_Mouth" "Fun"))
      (bind _returnvalue_4 (`KismetMaterialLibrary.GetVectorParameterValue` "/Game/_Resource/Monster/Lamball/MPC_Eye.MPC_Eye" "Fun"))
      (`MaterialInstanceDynamic.SetVectorParameterValue` (`self.MouseMaterial`) "Mouth" _returnvalue_3)
      (`MaterialInstanceDynamic.SetVectorParameterValue` (`self.EyeMaterial`) "Eye" _returnvalue_4))
    (:`2`
      (bind _returnvalue_5 (`KismetMaterialLibrary.GetVectorParameterValue` "/Game/_Resource/Monster/Lamball/MPC_Mouth.MPC_Mouth" "Ouch"))
      (bind _returnvalue_6 (`KismetMaterialLibrary.GetVectorParameterValue` "/Game/_Resource/Monster/Lamball/MPC_Eye.MPC_Eye" "Die"))
      (`MaterialInstanceDynamic.SetVectorParameterValue` (`self.MouseMaterial`) "Mouth" _returnvalue_5)
      (`MaterialInstanceDynamic.SetVectorParameterValue` (`self.EyeMaterial`) "Eye" _returnvalue_6))
    (:`3`
      (bind _returnvalue_7 (`KismetMaterialLibrary.GetVectorParameterValue` "/Game/_Resource/Monster/Lamball/MPC_Mouth.MPC_Mouth" "Sad"))
      (bind _returnvalue_8 (`KismetMaterialLibrary.GetVectorParameterValue` "/Game/_Resource/Monster/Lamball/MPC_Eye.MPC_Eye" "Sad"))
      (`MaterialInstanceDynamic.SetVectorParameterValue` (`self.MouseMaterial`) "Mouth" _returnvalue_7)
      (`MaterialInstanceDynamic.SetVectorParameterValue` (`self.EyeMaterial`) "Eye" _returnvalue_8))))

(fn `UserConstructionScript`
  (bind _mesh (`self.Mesh`))
  (bind _returnvalue (`PrimitiveComponent.CreateDynamicMaterialInstance` _mesh 0 null "None"))
  (set `self.EyeMaterial` _returnvalue)
  (bind _returnvalue_2 (`PrimitiveComponent.CreateDynamicMaterialInstance` _mesh 1 null "None"))
  (set `self.MouseMaterial` _returnvalue_2))