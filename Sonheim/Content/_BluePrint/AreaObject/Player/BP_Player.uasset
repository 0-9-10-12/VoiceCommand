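; Player Blueprint that uses hotkeys to issue AI voice orders for mining and lumbering, with no voice input wired in.
; Number and function keys call HandleAIVoiceOrder with preset actor, work and target values, some flagged as forced.
; Unconnected leftovers hold gather-to-player orders and submix recording to a WAV file.
; BeginPlay, Tick, overlap and construction logic are empty.
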(event `Key|F`
  (params (Key :type "Key Structure")))

(event `Key|One`
  (params (Key :type "Key Structure"))
  (:`Pressed`
    (`self.HandleAIVoiceOrder` (make `AIVoiceOrder` "Lamball" "Mining" "Stone"))))

(event `Key|Two`
  (params (Key :type "Key Structure"))
  (:`Pressed`
    (`self.HandleAIVoiceOrder` (make `AIVoiceOrder` "Anyone" "Mining" "Ore"))))

(event `Key|F1`
  (params (Key :type "Key Structure"))
  (:`Pressed`
    (`self.HandleAIVoiceOrder` (make `AIVoiceOrder` "Everyone" "Lumbering" "Tree" true))))

(event `Key|Three`
  (params (Key :type "Key Structure"))
  (:`Pressed`
    (`self.HandleAIVoiceOrder` (make `AIVoiceOrder` "Everyone" "Lumbering" "Tree" true))))

(event `Key|F2`
  (params (Key :type "Key Structure"))
  (:`Pressed`
    (`self.HandleAIVoiceOrder` (make `AIVoiceOrder` "Everyone" "Mining" "Stone" true))))

(event `Key|F3`
  (params (Key :type "Key Structure"))
  (:`Pressed`
    (`self.HandleAIVoiceOrder` (make `AIVoiceOrder` "Everyone" "Mining" "Ore" true))))

(event `Key|Four`
  (params (Key :type "Key Structure")))

(event `Key|Five`
  (params (Key :type "Key Structure")))

(event `Key|Six`
  (params (Key :type "Key Structure")))

(fn `UserConstructionScript`)